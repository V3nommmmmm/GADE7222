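; Bot1 is an AI bot Blueprint that tracks its own health and flags when it spots the player.
; AnyDamage subtracts from BotHealth, printing the remaining value or printing "Dead" and destroying the actor at zero or below.
; PawnSensing sets the "foundplayer" Blackboard bool to true on seeing a FirstPersonCharacter, with nothing here clearing it.
; The X key calls ApplyDamage on itself with no damage amount set.
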(event `self.ReceiveAnyDamage`
  (params (Damage :type "Float (single-precision)") (DamageType :type "DamageType Object Reference") (InstigatedBy :type "Controller Object Reference") (DamageCauser :type "Actor Object Reference"))
  (set `self.BotHealth` (- (`self.BotHealth`) Damage))
  (if (<= (`self.BotHealth`) 0.0)
    (`KismetSystemLibrary.PrintString` "Dead")
    (`self.K2_DestroyActor`)
    (else
      (`KismetSystemLibrary.PrintString` (`KismetStringLibrary.Conv_DoubleToString` (`self.BotHealth`))))))

(event `Key|X`
  (params (Key :type "Key Structure"))
  (:`Pressed`
    (`GameplayStatics.ApplyDamage` self)))

(event `self.PawnSensing.OnSeePawn`
  (params (Pawn :type "Pawn Object Reference"))
  (cast `/Game/Blueprints/FirstPersonCharacter` Pawn)
  (`BlackboardComponent.SetValueAsBool` (`AIBlueprintHelperLibrary.GetBlackboard` null) "foundplayer" true))

(fn `UserConstructionScript`)